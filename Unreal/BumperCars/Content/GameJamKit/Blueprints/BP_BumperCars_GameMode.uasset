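; Game mode for a local multiplayer bumper cars game that spawns player vehicles and handles the pause screen.
; On BeginPlay it gathers PlayerStarts, then creates a player and possessed vehicle for each count in the game instance.
; SetPause toggles the requesting player's pause widget, focusing Resume for player 0.
; It also writes each vehicle's SetGamePaused flag, true on removing the widget and false on showing it.
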(event Custom|SpawnPlayers
  (for _index (range 0 (- (Variables|/Game/GameJamKit/Blueprints/BP_BumperCars_GameInstance.BP_BumperCars_GameInstance_C|GetPlayerCountInstance (Variables|Default|GetGameInstanceRef)) 1))
    (Class|GameplayStatics|CreatePlayer _index)
    (bind _returnvalue (Game|SpawnActorfromClass "/Game/GameObjects/Vehicle/Vehicle.Vehicle_C" (Transformation|GetActorTransform (Utilities|Array|Get(acopy) (Variables|Default|GetPlayerStarts) _index)) "Undefined" 0 0))
    (Utilities|Array|AddUnique (Variables|Default|GetAllVehicles) _returnvalue)
    (Pawn|Possess (Game|GetPlayerController _index) _returnvalue)))

(event EventBeginPlay
  (CallFunction|GetAllStartPoints)
  (bind _asbp_bumper_cars_game_instance (Utilities|Casting|CastToBP_BumperCars_GameInstance (Game|GetGameInstance)))
  (Variables|Default|SetGameInstanceRef _asbp_bumper_cars_game_instance)
  (CallFunction|SpawnPlayers))

(event EventSetPause
  (params (ControllerID :type Integer))
  (Utilities|IsValid (Variables|Default|GetPauseScreenRef)
    (:Is%20Valid
      (Widget|RemovefromParent (Variables|Default|GetPauseScreenRef))
      (Variables|Default|SetPauseScreenRef 0)
      (for _array_element (Variables|Default|GetAllVehicles)
        (Variables|/Game/GameObjects/Vehicle/Vehicle.Vehicle_C|SetSetGamePaused _array_element true)))
    (:Is%20Not%20Valid
      (bind _returnvalue (UserInterface|CreateWidget "/Game/GameJamKit/Blueprints/UMG/PauseScreen.PauseScreen_C" (Game|GetPlayerController ControllerID)))
      (bind _output_get (Variables|Default|SetPauseScreenRef _returnvalue))
      (UserInterface|Viewport|AddtoPlayerScreen _output_get)
      (Class|Widget|SetUserFocus (Variables|/Game/GameJamKit/Blueprints/UMG/PauseScreen.PauseScreen_C|GetResumeButton _output_get) (Game|GetPlayerController 0))
      (for _array_element_2 (Variables|Default|GetAllVehicles)
        (Variables|/Game/GameObjects/Vehicle/Vehicle.Vehicle_C|SetSetGamePaused _array_element_2 false)))))

(fn ConstructionScript)

(fn GetAllStartPoints
  (bind _outactors (Actor|GetAllActorsOfClass "/Script/Engine.PlayerStart"))
  (Variables|Default|SetPlayerStarts _outactors)
  (return))