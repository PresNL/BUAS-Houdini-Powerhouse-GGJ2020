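; Wheel attachment that swaps the parent actor's current wheels for a set of four speed wheels.
; OnCreate destroys attached actors whose socket name contains "wheel", breaking and restarting the loop after each removal.
; It then spawns left and right speed-wheel actors, makes them movable and attaches them to the front and back wheel sockets.
; The attachment destroys itself afterwards, acting only as a one-shot installer.
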(event EventBeginPlay)

(event Collision|EventActorBeginOverlap
  (params (OtherActor :type Actor%20Object%20Reference))
  (|CallParentFunction OtherActor) ; This node is disabled and will not be called.\nDrag off pins to build functionality.
)

(event EventTick
  (params (DeltaSeconds :type Float%20%28single-precision%29))
  (|CallParentFunction DeltaSeconds) ; This node is disabled and will not be called.\nDrag off pins to build functionality.
)

(fn ConstructionScript
  (|CallParentFunction))

(fn OnCreate
  (params (parent :type Actor%20Object%20Reference))
  (Utilities|FlowControl|Sequence
    (:then_0
      (bind _array_element (Utilities|Array|ForEachLoopwithBreak (Actor|GetAttachedActors parent true) :!label _label)
        (:LoopBody
          (if (Utilities|String|Contains (Utilities|String|ToString(Name) (Class|Actor|GetAttachParentSocketName _array_element)) "wheel")
            (Actor|DestroyActor _array_element)
            (Utilities|FlowControl|Sequence
              (:then_0
                (goto _label Break))
              (:then_1
                (goto _label)))))))
    (:then_1
      (Utilities|FlowControl|Sequence
        (:then_0
          (bind _returnvalue (Game|SpawnActorfromClass "/Game/GameObjects/Attachment/Wheels/BP_wheel_speed_left.BP_wheel_speed_left_C" (Math|Transform|MakeTransform "0, 0, 0") "AlwaysSpawn" 0 0))
          (Transformation|SetMobility (Variables|/Script/Engine.Actor|GetRootComponent _returnvalue) "Movable")
          (Transformation|AttachActorToActor _returnvalue parent "left_back_wheel_right" "KeepRelative" "KeepRelative" "KeepRelative" true))
        (:then_1
          (bind _returnvalue_2 (Game|SpawnActorfromClass "/Game/GameObjects/Attachment/Wheels/BP_wheel_speed_left.BP_wheel_speed_left_C" (Math|Transform|MakeTransform "0, 0, 0") "AlwaysSpawn" 0 0))
          (Transformation|SetMobility (Variables|/Script/Engine.Actor|GetRootComponent _returnvalue_2) "Movable")
          (Transformation|AttachActorToActor _returnvalue_2 parent "left_front_wheel_right" "KeepRelative" "KeepRelative" "KeepRelative" true))
        (:then_2
          (bind _returnvalue_3 (Game|SpawnActorfromClass "/Game/GameObjects/Attachment/Wheels/BP_wheel_speed_right.BP_wheel_speed_right_C" (Math|Transform|MakeTransform "0, 0, 0") "AlwaysSpawn" 0 0))
          (Transformation|SetMobility (Variables|/Script/Engine.Actor|GetRootComponent _returnvalue_3) "Movable")
          (Transformation|AttachActorToActor _returnvalue_3 parent "right_back_wheel_right" "KeepRelative" "KeepRelative" "KeepRelative" true))
        (:then_3
          (bind _returnvalue_4 (Game|SpawnActorfromClass "/Game/GameObjects/Attachment/Wheels/BP_wheel_speed_right.BP_wheel_speed_right_C" (Math|Transform|MakeTransform "0, 0, 0") "AlwaysSpawn" 0 0))
          (Transformation|SetMobility (Variables|/Script/Engine.Actor|GetRootComponent _returnvalue_4) "Movable")
          (Transformation|AttachActorToActor _returnvalue_4 parent "right_front_wheel_right" "KeepRelative" "KeepRelative" "KeepRelative" true))
        (:then_4
          (Actor|DestroyActor))))))