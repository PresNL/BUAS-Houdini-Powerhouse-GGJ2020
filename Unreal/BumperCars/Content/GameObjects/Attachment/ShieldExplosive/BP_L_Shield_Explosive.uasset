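; Explosive shield attachment Blueprint that sets off an explosion when it is hit.
; Its OnHit override spawns an Explosionn actor 50 units from the shield, opposite the collision direction, then passes the hit to the parent implementation.
; All other behavior comes from the parent class, as the event graph holds only disabled default events and construction just calls the parent.
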(event EventBeginPlay
  (|CallParentFunction) ; This node is disabled and will not be called.\nDrag off pins to build functionality.
)

(event Collision|EventActorBeginOverlap
  (params (OtherActor :type Actor%20Object%20Reference))
  (|CallParentFunction OtherActor) ; This node is disabled and will not be called.\nDrag off pins to build functionality.
)

(event EventTick
  (params (DeltaSeconds :type Float%20%28single-precision%29))
  (|CallParentFunction DeltaSeconds) ; This node is disabled and will not be called.\nDrag off pins to build functionality.
)

(fn ConstructionScript
  (|CallParentFunction))

(fn OnHit
  (params (collisiondir :type Vector :default "0, 0, 0") (velocity :type Float%20%28single-precision%29) (other :type Actor%20Object%20Reference))
  (Game|SpawnActorfromClass "/Game/Blueprints/Explosion/Explosionn.Explosionn_C" (Math|Transform|MakeTransform (- (Transformation|GetActorLocation) (* collisiondir 5e+01)) "0, 0, 0" "1,1,1") "Undefined" 0 0)
  (|CallParentFunction collisiondir velocity other))