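; Base actor for vehicle attachments that exchange collision damage and play a sound on creation.
; Collider overlaps call OnHit on the other attachment or Vehicle, passing the direction and that actor's speed along it.
; OnHit subtracts speed-scaled damage plus any attacking attachment's BonusDamage from Health.
; It then destroys itself if Health is zero or above (seemingly inverted), otherwise applies an impulse to its parent Vehicle.
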(event OnComponentBeginOverlap(collider)
  (params (OverlappedComponent :type Primitive%20Component%20Object%20Reference) (OtherActor :type Actor%20Object%20Reference) (OtherComp :type Primitive%20Component%20Object%20Reference) (OtherBodyIndex :type Integer) (bFromSweep :type Boolean) (SweepResult :type Hit%20Result%20Structure%20%28by%20ref%29))
  (bind _returnvalue (Transformation|GetVelocity OtherActor))
  (bind _returnvalue_2 (Transformation|GetActorLocation))
  (bind _returnvalue_3 (Transformation|GetActorLocation OtherActor))
  (bind _returnvalue_4 (- _returnvalue_3 _returnvalue_2))
  (bind _returnvalue_5 (Math|Vector|Normalize _returnvalue_4))
  (bind _returnvalue_6 (Math|Vector|DotProduct _returnvalue _returnvalue_5))
  (bind _returnvalue_7 (Math|Float|Absolute(Float) _returnvalue_6))
  (bind _asbp_base_attachment (Utilities|Casting|CastToBP_BaseAttachment OtherActor)
    (:then
      (CallFunction|OnHit _asbp_base_attachment _returnvalue_5 _returnvalue_7 self))
    (:CastFailed
      (bind _asvehicle (Utilities|Casting|CastToVehicle OtherActor))
      (Default|OnHit _asvehicle _returnvalue_5 _returnvalue_7 self))))

(event OnComponentHit(collider)
  (params (HitComponent :type Primitive%20Component%20Object%20Reference) (OtherActor :type Actor%20Object%20Reference) (OtherComp :type Primitive%20Component%20Object%20Reference) (NormalImpulse :type Vector :default "0, 0, 0") (Hit :type Hit%20Result%20Structure%20%28by%20ref%29)))

(event EventBeginPlay)

(event Collision|EventActorBeginOverlap
  (params (OtherActor :type Actor%20Object%20Reference)))

(event EventTick
  (params (DeltaSeconds :type Float%20%28single-precision%29)))

(fn ConstructionScript)

(fn OnCreate
  (params (parent :type Actor%20Object%20Reference))
  (Audio|PlaySoundatLocation "/Game/Audio/Cues/S_Part_Attach_Cue.S_Part_Attach_Cue" (Transformation|GetActorLocation parent) "0, 0, 0" 1.0 1.0 0.0 0 0 0))

(fn OnHit
  (params (collisiondir :type Vector) (velocity :type Float%20%28single-precision%29) (other :type Actor%20Object%20Reference))
  (bind _returnvalue (* velocity 0.0001))
  (bind _asbp_base_attachment (Utilities|Casting|CastToBP_BaseAttachment other)
    (:then
      (Variables|Default|Sethealth (- (Variables|Default|Gethealth) (+ _returnvalue (Variables|BP_BaseAttachment_C|GetbonusDamage _asbp_base_attachment)))))
    (:CastFailed
      (Variables|Default|Sethealth (- (Variables|Default|Gethealth) _returnvalue))))
  (if (<= 0.0 (Variables|Default|Gethealth))
    (Actor|DestroyActor)
    (else
      (bind _asvehicle (Utilities|Casting|CastToVehicle (Actor|GetAttachParentActor)))
      (Default|ApplyImpulseatPosition _asvehicle false collisiondir (* velocity 5e+01)))))