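; Base pickup that grants an Attachment class to a Vehicle that overlaps it.
; On BeginPlay it briefly spawns the attachment to read its attachment point, mesh and first material, copies the visuals onto an attached collisionless mesh actor, and sizes its box from the mesh bounds.
; On overlap, if the vehicle has nothing attached at that socket, it calls PickupItem with the class, then destroys itself and its display mesh.
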(event EventBeginPlay
  (bind _returnvalue (Math|Transform|MakeTransform "0, 0, 0"))
  (bind _returnvalue_2 (Game|SpawnActorfromClass (Variables|Default|Getattachment) _returnvalue "AlwaysSpawn" 0 0))
  (Variables|Default|SetattachmentPoint (Variables|/Game/GameObjects/Attachment/BP_BaseAttachment.BP_BaseAttachment_C|GetattachmentPoint _returnvalue_2))
  (bind _returnvalue_3 (Game|SpawnActorfromClass "/Script/Engine.StaticMeshActor" _returnvalue "Undefined" 0 0))
  (Transformation|SetMobility _returnvalue_3 "Movable")
  (Collision|SetCollisionEnabled (Variables|/Script/Engine.StaticMeshActor|GetStaticMeshComponent _returnvalue_3) "NoCollision")
  (Components|StaticMesh|SetStaticMesh (Variables|/Script/Engine.StaticMeshActor|GetStaticMeshComponent _returnvalue_3) (Variables|/Script/Engine.StaticMeshComponent|GetStaticMesh (Actor|GetComponentbyClass _returnvalue_2 "/Script/Engine.StaticMeshComponent")))
  (Rendering|Material|SetMaterial (Variables|/Script/Engine.StaticMeshActor|GetStaticMeshComponent _returnvalue_3) 0 (Rendering|Material|GetMaterial (Actor|GetComponentbyClass _returnvalue_2 "/Script/Engine.StaticMeshComponent") 0))
  (Transformation|AttachActorToActor _returnvalue_3 self "None" "KeepRelative" "KeepRelative" "KeepRelative" true)
  (Components|Box|SetBoxExtent (Actor|GetComponentbyClass "/Script/Engine.BoxComponent") (- (.Max (Components|StaticMesh|GetLocalBounds (Actor|GetComponentbyClass _returnvalue_3 "/Script/Engine.StaticMeshComponent"))) (.Min (Components|StaticMesh|GetLocalBounds (Actor|GetComponentbyClass _returnvalue_3 "/Script/Engine.StaticMeshComponent")))) true)
  (Actor|DestroyActor _returnvalue_2))

(event Collision|EventActorBeginOverlap
  (params (OtherActor :type Actor%20Object%20Reference))
  (Variables|Default|Setbreak false)
  (bind _asvehicle (Utilities|Casting|CastToVehicle OtherActor))
  (bind _array_element (Utilities|Array|ForEachLoopwithBreak (Actor|GetAttachedActors _asvehicle true) :!label _label)
    (:LoopBody
      (if (Utilities|Enum|Equal(Enum) (Utilities|String|ToString(Name) (Class|Actor|GetAttachParentSocketName _array_element)) (Variables|Default|GetattachmentPoint))
        (Variables|Default|Setbreak true)
        (goto _label Break)))
    (:Completed
      (if (not (Variables|Default|Getbreak))
        (Default|PickupItem _asvehicle (Variables|Default|Getattachment))
        (for _array_element_2 (Actor|GetAttachedActors true)
          (Actor|DestroyActor _array_element_2))
        (Actor|DestroyActor)))))

(event EventTick
  (params (DeltaSeconds :type Float%20%28single-precision%29)))

(fn ConstructionScript)