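; Shared multiplayer camera actor that follows the centroid of all player pawns and zooms to keep them on screen.
; Each tick it lerps its XY toward the centroid, faster beyond LazyDistance, and keeps its height.
; If any player, projected through player 0's view, leaves the viewport margins, ZoomTarget steps back; otherwise it steps forward.
; The Camera component eases along local X toward that target, capped at zero.
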(event EventBeginPlay)

(event EventTick
  (params (DeltaSeconds :type Float%20%28single-precision%29))
  (bind _centroid (CallFunction|GetPlayerCentroid))
  (bind _returnvalue (Transformation|GetActorLocation))
  (bind _zoomspeed (Variables|Default|GetZoomSpeed))
  ;[1 1 1] Setting location
  ;;[1 1 1] Comment
  (Utilities|FlowControl|Sequence
    (:then_0
      (if (>= (Math|Vector|VectorLengthSquared (- _returnvalue _centroid)) (Math|Float|Square (Variables|Default|GetLazyDistance)))
        (Variables|Default|SetLerpSpeed 0.1)
        (else
          (Variables|Default|SetLerpSpeed 0.01))))
    (:then_1
      (Transformation|SetActorLocation (Math|Vector|MakeVector (.x (Math|Vector|Lerp(Vector) _returnvalue _centroid (Variables|Default|GetLerpSpeed))) (.y (Math|Vector|Lerp(Vector) _returnvalue _centroid (Variables|Default|GetLerpSpeed))) (.z (Transformation|GetActorLocation))) false false)
      (if (CallFunction|GetFurthestPlayerDistancefromEdge)
        (Variables|Default|SetZoomTarget (- (Variables|Default|GetZoomTarget) _zoomspeed))
        (Utilities|LerptoZoomTarget 0.1)
        (else
          (Variables|Default|SetZoomTarget (+ (Variables|Default|GetZoomTarget) _zoomspeed))
          (Utilities|LerptoZoomTarget 0.1))))))

(fn ConstructionScript)

(fn GetPlayerCentroid
  (bind _returnvalue (Class|GameModeBase|GetNumPlayers (Game|GetGameMode)))
  (for _index (range 0 (- _returnvalue 1))
    (LocalVariables|SetAccumulator (+ (Transformation|GetActorLocation (Game|Player|GetPlayerPawn _index)) (LocalVariables|GetAccumulator))))
  (return (/ (LocalVariables|GetAccumulator) _returnvalue)))

(fn GetFurthestPlayerDistancefromEdge
  (bind _returnvalue (Class|GameModeBase|GetNumPlayers (Game|GetGameMode)))
  (for _index (range 0 (- _returnvalue 1))
    (bind (_p1 _p2) (CallFunction|CalcBoundingBox (Math|Vector2D|MakeVector2D (Variables|Default|GetHorizontalMargin) (Variables|Default|GetVerticalMargin))))
    (bind _outofbounds (CallFunction|IsOutOfBounds (Math|Vector2D|MakeVector2D (.x (.ScreenPosition (Class|GameplayStatics|ProjectWorldtoScreen (Game|GetPlayerController 0) (Transformation|GetActorLocation (Game|Player|GetPlayerPawn _index)) false))) (.y (.ScreenPosition (Class|GameplayStatics|ProjectWorldtoScreen (Game|GetPlayerController 0) (Transformation|GetActorLocation (Game|Player|GetPlayerPawn _index)) false)))) _p1 _p2))
    (if _outofbounds
      (return true)))
  (return false))

(fn GetDistancefromMargin
  (params (AxisValue :type Float%20%28single-precision%29) (AxisMargin :type Float%20%28single-precision%29) (AxisSize :type Float%20%28single-precision%29))
  (return (select (< AxisValue (/ AxisSize 2.0)) (- AxisValue AxisMargin) (* (- AxisValue (- AxisSize AxisMargin)) -1.0))))

(fn CalcBoundingBox
  (params (Margins :type Vector%202D%20Structure))
  (bind _returnvalue (Viewport|GetViewportSize))
  (bind _returnvalue_2 (* (.x Margins) (.x _returnvalue)))
  (bind _returnvalue_3 (* (.y Margins) (.y _returnvalue)))
  (return (Math|Vector2D|MakeVector2D _returnvalue_2 _returnvalue_3) (Math|Vector2D|MakeVector2D (- (.x _returnvalue) _returnvalue_2) (- (.y _returnvalue) _returnvalue_3))))

(fn IsOutOfBounds
  (params (P0 :type Vector%202D%20Structure) (Min :type Vector%202D%20Structure) (Max :type Vector%202D%20Structure))
  (return (Math|Boolean|ORBoolean (< (.x P0) (.x Min)) (> (.x P0) (.x Max)) (< (.y P0) (.y Min)) (> (.y P0) (.y Max)))))