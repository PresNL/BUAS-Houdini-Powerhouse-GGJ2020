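; BP_SoundTest is an audio test Blueprint that simulates engine sound driven by holding and releasing the Up key.
; Idle starts on BeginPlay, then sine-curve fades crossfade between idle, rev-up, high loop and rev-down sounds.
; Two timelines track rev progress, triggering the high loop and the return to idle.
; Their positions set audio start offsets, mirrored over seven seconds for rev-down, so interrupted revs resume at corresponding points.
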(event EventBeginPlay
  (Input|EnableInput (Game|GetPlayerController 0))
  ;[1 1 1] Starts Engine Idle Loop at start play
  (Audio|Components|Audio|Play (Variables|Default|GetEngine%20Idle) 0.0))

(event Input|KeyboardEvents|Up
  (params (Key :type Key%20Structure :default "None"))
  (:Pressed
    (Utilities|FlowControl|Sequence
      (:then_0
        (bind _time (Timeline|Timer SetNewTime)
          (:Trigger%20High%20Loop
            (Audio|Components|Audio|FadeOut (Variables|Default|GetEngine%20Rev) 0.2 0.0 "Sin" :!class /Script/Engine.AudioComponent)
            (Audio|Components|Audio|FadeIn (Variables|Default|GetEngine%20High) 0.2 1.0 0.0 "Sin" :!class /Script/Engine.AudioComponent))))
      (:then_1
        (Timeline|Timer Play))
      (:then_2
        (bind _time_2 (Timeline|RevDown%20Timer Stop)
          (:Finished
            (Audio|Components|Audio|FadeOut (Variables|Default|GetEngine%20RevDown) 0.2 0.0 "Sin" :!class /Script/Engine.AudioComponent)
            (Audio|Components|Audio|FadeIn (Variables|Default|GetEngine%20Idle) 0.2 1.0 0.0 "Sin" :!class /Script/Engine.AudioComponent))))
      (:then_3
        (Audio|Components|Audio|FadeIn (Variables|Default|GetEngine%20Rev) 0.2 1.0 _time "Sin" :!class /Script/Engine.AudioComponent)
        (Audio|Components|Audio|FadeOut (Variables|Default|GetEngine%20Idle) 0.2 0.0 "Sin" :!class /Script/Engine.AudioComponent)
        (Audio|Components|Audio|FadeOut (Variables|Default|GetEngine%20RevDown) 0.2 0.0 "Sin" :!class /Script/Engine.AudioComponent))))
  (:Released
    (Utilities|FlowControl|Sequence
      (:then_0
        (Timeline|Timer Stop))
      (:then_1
        (Audio|Components|Audio|FadeOut (Variables|Default|GetEngine%20Rev) 0.2 0.0 "Sin" :!class /Script/Engine.AudioComponent)
        (Audio|Components|Audio|FadeIn (Variables|Default|GetEngine%20RevDown) 0.2 1.0 (- 7.0 _time) "Sin" :!class /Script/Engine.AudioComponent)
        (Utilities|FlowControl|Sequence
          (:then_0
            (Audio|Components|Audio|FadeOut (Variables|Default|GetEngine%20High) 0.2 0.0 "Sin" :!class /Script/Engine.AudioComponent)
            (Audio|Components|Audio|FadeOut (Variables|Default|GetEngine%20Rev) 0.2 0.0 "Sin" :!class /Script/Engine.AudioComponent))
          (:then_1
            (Timeline|RevDown%20Timer PlayFromStart))))
      (:then_2
        (Timeline|RevDown%20Timer SetNewTime)))))

(fn ConstructionScript)